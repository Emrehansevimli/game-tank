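; Land mine actor that explodes when a BP_BasePawn enters its trigger sphere or when it takes any damage.
; Both events share one sequence: click sound, half-second delay, damage to the pawn cast from the overlap, explosion effect and sound, then self-destruction.
; The damage amount comes from the AnyDamage event, with no value set on the overlap path.
; Tick flashes a point light through a short Delay.
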(event OnComponentBeginOverlap(Sphere)
  (params (OverlappedComponent :type Primitive%20Component%20Object%20Reference) (OtherActor :type Actor%20Object%20Reference) (OtherComp :type Primitive%20Component%20Object%20Reference) (OtherBodyIndex :type Integer) (bFromSweep :type Boolean) (SweepResult :type Hit%20Result%20Structure%20%28by%20ref%29))
  (bind _asbp_base_pawn (Utilities|Casting|CastToBP_BasePawn OtherActor))
  (Audio|SpawnSoundAttached "/Engine/VREditor/Sounds/UI/Click_on_Button.Click_on_Button" (Variables|Default|GetStaticMesh) "None" "0, 0, 0" "0, 0, 0" "KeepRelativeOffset" false 1.0 1.0 0.0 0 0)
  (Utilities|FlowControl|Delay 0.5)
  (Game|Damage|ApplyDamage _asbp_base_pawn (stale Game|Damage|EventAnyDamage _output_get) 0 self)
  (Effects|SpawnEmitteratLocation "/Game/StarterContent/Particles/P_Explosion.P_Explosion" (Transformation|GetWorldLocation (Variables|Default|GetStaticMesh)) "0, 0, 0" "10.000000,10.000000,10.000000")
  (Audio|SpawnSoundAttached "/Game/StarterContent/Audio/Explosion01.Explosion01" (Variables|Default|GetStaticMesh) "None" "0, 0, 0" "0, 0, 0" "KeepRelativeOffset" false 1.0 1.0 0.0 0 0)
  (Actor|DestroyActor))

(event Game|Damage|EventAnyDamage
  (params (Damage :type Float%20%28single-precision%29) (DamageType :type Damage%20Type%20Object%20Reference) (InstigatedBy :type Controller%20Object%20Reference) (DamageCauser :type Actor%20Object%20Reference))
  (bind _output_get (Variables|Default|Setdamage Damage))
  (Audio|SpawnSoundAttached "/Engine/VREditor/Sounds/UI/Click_on_Button.Click_on_Button" (Variables|Default|GetStaticMesh) "None" "0, 0, 0" "0, 0, 0" "KeepRelativeOffset" false 1.0 1.0 0.0 0 0)
  (Utilities|FlowControl|Delay 0.5)
  (Game|Damage|ApplyDamage (stale OnComponentBeginOverlap(Sphere) _asbp_base_pawn) _output_get 0 self)
  (Effects|SpawnEmitteratLocation "/Game/StarterContent/Particles/P_Explosion.P_Explosion" (Transformation|GetWorldLocation (Variables|Default|GetStaticMesh)) "0, 0, 0" "10.000000,10.000000,10.000000")
  (Audio|SpawnSoundAttached "/Game/StarterContent/Audio/Explosion01.Explosion01" (Variables|Default|GetStaticMesh) "None" "0, 0, 0" "0, 0, 0" "KeepRelativeOffset" false 1.0 1.0 0.0 0 0)
  (Actor|DestroyActor))

(event EventTick
  (params (DeltaSeconds :type Float%20%28single-precision%29))
  (Variables|Default|SetDelta%20Seconds DeltaSeconds)
  (Rendering|Components|Light|SetIntensity (Variables|Default|GetPointLight) 0.0)
  (Utilities|FlowControl|Delay 0.2)
  (Rendering|Components|Light|SetIntensity (Variables|Default|GetPointLight) 6e+03))

(fn ConstructionScript)