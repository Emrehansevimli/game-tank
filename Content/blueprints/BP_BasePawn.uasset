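; Player tank pawn with mobile touch controls that tracks health, wallet money and level progress.
; BeginPlay shows the left virtual joystick and tank HUD, then loads the "save1" slot or calls Save if none exists.
; Damage reduces Can (health); at exactly zero the pawn is destroyed and a death screen takes UI-only input.
; Save writes money and finished level, raising the stored max level, only when RefSave is valid.
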(event EventBeginPlay
  (Class|PlayerController|ActivateTouchInterface (Game|GetPlayerController 0) "/Engine/MobileResources/HUD/LeftVirtualJoystickOnly.LeftVirtualJoystickOnly")
  (bind _returnvalue (UserInterface|CreateWidget "/Game/blueprints/tank_WİDGETBP.tank_WİDGETBP_C"))
  (UserInterface|Viewport|AddtoPlayerScreen _returnvalue)
  ;[1 1 1] save system
  (bind _returnvalue_2 (SaveGame|DoesSaveGameExist "save1"))
  (if _returnvalue_2
    (CallFunction|Load)
    (else
      (CallFunction|Save))))

(event Game|Damage|EventAnyDamage
  (params (Damage :type Float%20%28single-precision%29) (DamageType :type Damage%20Type%20Object%20Reference) (InstigatedBy :type Controller%20Object%20Reference) (DamageCauser :type Actor%20Object%20Reference))
  (bind _returnvalue (Game|GetPlayerController 0))
  (bind _output_get (Variables|Default|Setcan (- (Variables|Default|Getcan) Damage)))
  (if (== _output_get 0.0)
    (Class|PlayerController|ActivateTouchInterface (Game|GetPlayerController 0))
    (Actor|DestroyActor)
    (bind _returnvalue_2 (UserInterface|CreateWidget "/Game/blueprints/deadScreen_bp.deadScreen_bp_C"))
    (UserInterface|Viewport|AddtoPlayerScreen _returnvalue_2)
    (Input|SetInputModeUIOnly _returnvalue 0 "DoNotLock" false)
    (Variables|/Script/Engine.PlayerController|SetbShowMouseCursor _returnvalue true)))

(fn ConstructionScript)

(fn Load
  (bind _returnvalue (SaveGame|LoadGamefromSlot "save1"))
  (bind _asbp_save (Utilities|Casting|CastTobp_save _returnvalue))
  (Variables|Default|Setref%20save _asbp_save)
  (Variables|Default|Setwallet (Variables|/Game/blueprints/bp_save.bp_save_C|Getmoney _asbp_save))
  (Variables|Default|Setlevel_finish (Variables|/Game/blueprints/bp_save.bp_save_C|Getfinish_level (Variables|Default|Getref%20save))))

(fn Save
  (bind _ref_save (Variables|Default|Getref%20save))
  (bind _ref_save_2 (Variables|Default|Getref%20save))
  (SaveGame|CreateSaveGameObject "/Game/blueprints/bp_save.bp_save_C")
  (Utilities|IsValid _ref_save_2
    (:Is%20Valid
      (Variables|/Game/blueprints/bp_save.bp_save_C|Setmoney _ref_save_2 (Variables|Default|Getwallet))
      (Variables|/Game/blueprints/bp_save.bp_save_C|Setfinish_level _ref_save (Variables|Default|Getlevel_finish))
      (if (< (Variables|/Game/blueprints/bp_save.bp_save_C|Getmaxlevel _ref_save) (Variables|Default|Getlevel_finish))
        (Variables|/Game/blueprints/bp_save.bp_save_C|Setmaxlevel (Variables|Default|Getref%20save) (Variables|Default|Getlevel_finish)))
      (SaveGame|SaveGametoSlot (Variables|Default|Getref%20save) "save1"))))