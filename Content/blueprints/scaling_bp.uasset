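; Scaling trigger actor that toggles an overlapping BP_BasePawn between small and big states through its Small and Big components.
; Each overlap multiplies the actor's relative scale onto the capsule, changes camera FOV and spawns a hit effect; growing also nudges the capsule upward.
; The pawn's IsSmallData flag blocks repeat triggers, and the grow factor is not the inverse of the shrink factor.
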(event OnComponentBeginOverlap(small)
  (params (OverlappedComponent :type Primitive%20Component%20Object%20Reference) (OtherActor :type Actor%20Object%20Reference) (OtherComp :type Primitive%20Component%20Object%20Reference) (OtherBodyIndex :type Integer) (bFromSweep :type Boolean) (SweepResult :type Hit%20Result%20Structure%20%28by%20ref%29))
  (bind _asbp_base_pawn (Utilities|Casting|CastToBP_BasePawn OtherActor))
  (if (not (Variables|/Game/blueprints/BP_BasePawn.BP_BasePawn_C|Getis%20small%20data _asbp_base_pawn))
    (Transformation|SetWorldScale3D (Variables|/Script/Proto4.BasePawn|GetCapsuleComp _asbp_base_pawn) (* (Class|Actor|GetActorRelativeScale3D _asbp_base_pawn) "0.500000,0.500000,0.500000"))
    (Camera|SetFieldOfView (Variables|/Script/Proto4.BasePawn|GetCameraComp _asbp_base_pawn) 7e+01)
    (Effects|SpawnEmitteratLocation "/Game/Assets/Effects/P_HitEffect.P_HitEffect" (Transformation|GetWorldLocation (Variables|Default|Getsmall)) "180.000000,0.000000,0.000000" "5.000000,5.000000,5.000000")
    (Variables|/Game/blueprints/BP_BasePawn.BP_BasePawn_C|Setis%20small%20data _asbp_base_pawn true)))

(event OnComponentBeginOverlap(big)
  (params (OverlappedComponent :type Primitive%20Component%20Object%20Reference) (OtherActor :type Actor%20Object%20Reference) (OtherComp :type Primitive%20Component%20Object%20Reference) (OtherBodyIndex :type Integer) (bFromSweep :type Boolean) (SweepResult :type Hit%20Result%20Structure%20%28by%20ref%29))
  (bind _asbp_base_pawn (Utilities|Casting|CastToBP_BasePawn OtherActor))
  (if (Variables|/Game/blueprints/BP_BasePawn.BP_BasePawn_C|Getis%20small%20data _asbp_base_pawn)
    (Transformation|SetWorldScale3D (Variables|/Script/Proto4.BasePawn|GetCapsuleComp _asbp_base_pawn) (* (Class|Actor|GetActorRelativeScale3D _asbp_base_pawn) "1.300000,1.300000,1.300000"))
    (Transformation|SetWorldLocation (Variables|/Script/Proto4.BasePawn|GetCapsuleComp _asbp_base_pawn) (Math|Vector|MakeVector (.x (Transformation|GetWorldLocation (Variables|/Script/Proto4.BasePawn|GetCapsuleComp _asbp_base_pawn))) (.y (Transformation|GetWorldLocation (Variables|/Script/Proto4.BasePawn|GetCapsuleComp _asbp_base_pawn))) (+ (.z (Transformation|GetWorldLocation (Variables|/Script/Proto4.BasePawn|GetCapsuleComp _asbp_base_pawn))) 1e+01)) false false)
    (Camera|SetFieldOfView (Variables|/Script/Proto4.BasePawn|GetCameraComp _asbp_base_pawn) 9e+01)
    (Effects|SpawnEmitteratLocation "/Game/Assets/Effects/P_HitEffect.P_HitEffect" (Transformation|GetWorldLocation (Variables|Default|Getbig)) "180.000000,0.000000,0.000000" "5.000000,5.000000,5.000000")
    (Variables|/Game/blueprints/BP_BasePawn.BP_BasePawn_C|Setis%20small%20data _asbp_base_pawn false)))

(event EventBeginPlay)

(event Collision|EventActorBeginOverlap
  (params (OtherActor :type Actor%20Object%20Reference)))

(event EventTick
  (params (DeltaSeconds :type Float%20%28single-precision%29)))

(fn ConstructionScript)