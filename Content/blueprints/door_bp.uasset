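; Key-operated door Blueprint whose Door1 component is moved by two timelines.
; The key's Sphere spins each tick while Open is false.
; When a BP_BasePawn overlaps the Sphere, it destroys Sphere, Key and TextRender, sets Open and plays one timeline.
; A BP_BasePawn overlapping Box1 while Open is false plays the other timeline, which sets the pawn's IsDoorClose flag.
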(event OnComponentBeginOverlap(Box1)
  (params (OverlappedComponent :type Primitive%20Component%20Object%20Reference) (OtherActor :type Actor%20Object%20Reference) (OtherComp :type Primitive%20Component%20Object%20Reference) (OtherBodyIndex :type Integer) (bFromSweep :type Boolean) (SweepResult :type Hit%20Result%20Structure%20%28by%20ref%29))
  (bind _asbp_base_pawn (Utilities|Casting|CastToBP_BasePawn OtherActor))
  (if (not (Variables|Default|Getopen))
    (bind _newtrack_1 (Timeline|Timeline_0 Play)
      (:Update
        (Transformation|SetRelativeLocation (Variables|Default|Getdoor1) (Math|Vector|MakeVector (.x _newtrack_1) (.y _newtrack_1) (.z _newtrack_1)) false false)
        (if (Utilities|IsValid _asbp_base_pawn)
          (Variables|/Game/blueprints/BP_BasePawn.BP_BasePawn_C|Setis%20door%20close _asbp_base_pawn true)
          (Variables|Default|Setopen false))))))

(event OnComponentBeginOverlap(Sphere)
  (params (OverlappedComponent :type Primitive%20Component%20Object%20Reference) (OtherActor :type Actor%20Object%20Reference) (OtherComp :type Primitive%20Component%20Object%20Reference) (OtherBodyIndex :type Integer) (bFromSweep :type Boolean) (SweepResult :type Hit%20Result%20Structure%20%28by%20ref%29))
  (Utilities|Casting|CastToBP_BasePawn OtherActor)
  (Components|DestroyComponent (Variables|Default|GetSphere))
  (Variables|Default|Setopen true)
  (bind _newtrack_1 (Timeline|Timeline Play)
    (:Update
      (Transformation|SetRelativeLocation (Variables|Default|Getdoor1) (Math|Vector|MakeVector (.x _newtrack_1) (.y _newtrack_1) (.z _newtrack_1)) false false))))

(event Collision|EventActorBeginOverlap
  (params (OtherActor :type Actor%20Object%20Reference)))

(event EventTick
  (params (DeltaSeconds :type Float%20%28single-precision%29))
  (if (not (Variables|Default|Getopen))
    (Transformation|AddRelativeRotation (Variables|Default|GetSphere) "0.000000,1.000000,0.000000" false false)))

(fn ConstructionScript)