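; BP_Enemy is an enemy that shifts its BaseMesh toward or away along local X in response to player overlaps.
; Once the player enters Sphere, Tick nudges the mesh by a fixed per-frame step, signed by the last Forwardbox or Backwardbox entered.
; Entering Sphere1 stops movement permanently, as no flag resets on end overlap.
; PawnSensing only sets a flag for FollowPlayer's AIMoveTo, which is called only from unwired nodes.
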(event OnSeePawn(PawnSensing)
  (params (Pawn :type Pawn%20Object%20Reference))
  (Variables|Default|SetIsSeenPlayer true))

(event OnComponentBeginOverlap(Sphere)
  (params (OverlappedComponent :type Primitive%20Component%20Object%20Reference) (OtherActor :type Actor%20Object%20Reference) (OtherComp :type Primitive%20Component%20Object%20Reference) (OtherBodyIndex :type Integer) (bFromSweep :type Boolean) (SweepResult :type Hit%20Result%20Structure%20%28by%20ref%29))
  (if (== OtherActor (Game|Player|GetPlayerPawn 0))
    (Variables|Default|SetIsEnteredSphere true)))

(event OnComponentBeginOverlap(forwardbox)
  (params (OverlappedComponent :type Primitive%20Component%20Object%20Reference) (OtherActor :type Actor%20Object%20Reference) (OtherComp :type Primitive%20Component%20Object%20Reference) (OtherBodyIndex :type Integer) (bFromSweep :type Boolean) (SweepResult :type Hit%20Result%20Structure%20%28by%20ref%29))
  (if (== OtherActor (Game|Player|GetPlayerPawn 0))
    (Variables|Default|SetIsforwardbox true)
    (Variables|Default|SetIsbackwardbox false)))

(event OnComponentBeginOverlap(Sphere1)
  (params (OverlappedComponent :type Primitive%20Component%20Object%20Reference) (OtherActor :type Actor%20Object%20Reference) (OtherComp :type Primitive%20Component%20Object%20Reference) (OtherBodyIndex :type Integer) (bFromSweep :type Boolean) (SweepResult :type Hit%20Result%20Structure%20%28by%20ref%29))
  (if (== OtherActor (Game|Player|GetPlayerPawn 0))
    (Variables|Default|SetIsCloseEnought true)
    (Development|PrintString "close")))

(event OnComponentBeginOverlap(backwardbox)
  (params (OverlappedComponent :type Primitive%20Component%20Object%20Reference) (OtherActor :type Actor%20Object%20Reference) (OtherComp :type Primitive%20Component%20Object%20Reference) (OtherBodyIndex :type Integer) (bFromSweep :type Boolean) (SweepResult :type Hit%20Result%20Structure%20%28by%20ref%29))
  (if (== OtherActor (Game|Player|GetPlayerPawn 0))
    (Variables|Default|SetIsbackwardbox true)
    (Variables|Default|SetIsforwardbox false)))

(event Custom|FollowPlayer
  (if (Variables|Default|GetIsSeenPlayer)
    (AI|AIMoveTo self "0, 0, 0" (Game|GetPlayerCharacter 0) 5.0 false
      (:OnSuccess
        (Development|PrintText "sucsess"))
      (:OnFail
        (Development|PrintText "fail")))))

(event EventBeginPlay)

(event Collision|EventActorBeginOverlap
  (params (OtherActor :type Actor%20Object%20Reference)))

(event EventTick
  (params (DeltaSeconds :type Float%20%28single-precision%29))
  (if (and (not (Variables|Default|GetIsCloseEnought)) (Variables|Default|GetIsEnteredSphere))
    (bind _asbase_pawn (Utilities|Casting|CastToBasePawn (stale OnComponentBeginOverlap(Sphere) OtherActor)))
    (Variables|Default|SetAs%20Base%20Pawn _asbase_pawn)
    (if (Variables|Default|GetIsforwardbox)
      (Transformation|AddLocalOffset (Variables|Default|GetBaseMesh) "2.000000,0.000000,0.000000" false false)
      (elif (Variables|Default|GetIsbackwardbox)
        (Transformation|AddLocalOffset (Variables|Default|GetBaseMesh) "-2.000000,0.000000,0.000000" false false)))))

(fn ConstructionScript)