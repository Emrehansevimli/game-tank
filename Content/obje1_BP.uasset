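; obje1_BP is a static mesh prop that gets knocked over when a BasePawn hits it.
; On hit, it snaps the DefaultSceneRoot to a -90 degree roll with a random yaw offset, keeping location, pitch and scale.
; The mesh then ignores the WorldDynamic channel and plays a thud sound at its location.
; The fall is an instant transform change, with no animation or physics impulse.
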(event OnComponentHit(StaticMesh)
  (params (HitComponent :type Primitive%20Component%20Object%20Reference) (OtherActor :type Actor%20Object%20Reference) (OtherComp :type Primitive%20Component%20Object%20Reference) (NormalImpulse :type Vector :default "0, 0, 0") (Hit :type Hit%20Result%20Structure%20%28by%20ref%29))
  (bind _defaultsceneroot (Variables|Default|GetDefaultSceneRoot))
  (bind _returnvalue (Transformation|GetWorldTransform _defaultsceneroot))
  (Utilities|Casting|CastToBasePawn OtherActor)
  (Transformation|SetWorldTransform (Variables|Default|GetDefaultSceneRoot) (Math|Transform|MakeTransform (.location _returnvalue) (Math|Rotator|MakeRotator -9e+01 (.pitch (.rotation _returnvalue)) (+ (.yaw (.rotation _returnvalue)) (Math|Conversions|ToFloat(Integer) (Math|Random|RandomIntegerinRange -30 30)))) (.scale _returnvalue)) false false)
  (Collision|SetCollisionResponsetoChannel (Variables|Default|GetStaticMesh) "ECC_WorldDynamic" "ECR_Ignore")
  (Audio|SpawnSoundatLocation "/Game/Assets/Audio/Thud_Audio.Thud_Audio" (Transformation|GetWorldLocation (Variables|Default|GetStaticMesh)) "0, 0, 0" 1.0 1.0 0.0 0 0))

(event EventBeginPlay)

(event Collision|EventActorBeginOverlap
  (params (OtherActor :type Actor%20Object%20Reference)))

(event EventTick
  (params (DeltaSeconds :type Float%20%28single-precision%29)))

(fn ConstructionScript)