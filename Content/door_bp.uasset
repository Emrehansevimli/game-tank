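; Door Blueprint with a key pickup that opens it and a trigger that shuts it.
; While the door is not open, Tick spins the key's Sphere.
; A BP_BasePawn overlapping the Sphere destroys the key components and instantly slides Door1 aside.
; Overlapping Box1 snaps the door back and clears Open, gated by the pawn's IsDoorClose flag, which it then sets to prevent repeats.
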(event OnComponentBeginOverlap(Box1)
  (params (OverlappedComponent :type Primitive%20Component%20Object%20Reference) (OtherActor :type Actor%20Object%20Reference) (OtherComp :type Primitive%20Component%20Object%20Reference) (OtherBodyIndex :type Integer) (bFromSweep :type Boolean) (SweepResult :type Hit%20Result%20Structure%20%28by%20ref%29))
  (bind _asbp_base_pawn (Utilities|Casting|CastToBP_BasePawn OtherActor))
  (if (not (Variables|/Game/BP_BasePawn.BP_BasePawn_C|Getis%20door%20close _asbp_base_pawn))
    (Transformation|SetRelativeLocation (Variables|Default|Getdoor1) "0.000000,9.542786,0.000000" false false)
    (Variables|/Game/BP_BasePawn.BP_BasePawn_C|Setis%20door%20close _asbp_base_pawn true)
    (Variables|Default|Setopen false)))

(event OnComponentBeginOverlap(Sphere)
  (params (OverlappedComponent :type Primitive%20Component%20Object%20Reference) (OtherActor :type Actor%20Object%20Reference) (OtherComp :type Primitive%20Component%20Object%20Reference) (OtherBodyIndex :type Integer) (bFromSweep :type Boolean) (SweepResult :type Hit%20Result%20Structure%20%28by%20ref%29))
  (Utilities|Casting|CastToBP_BasePawn OtherActor)
  (Components|DestroyComponent (Variables|Default|GetSphere))
  (Variables|Default|Setopen true)
  (Transformation|SetRelativeLocation (Variables|Default|Getdoor1) "-159.994775,9.542786,0.000000" false false))

(event Collision|EventActorBeginOverlap
  (params (OtherActor :type Actor%20Object%20Reference)))

(event EventTick
  (params (DeltaSeconds :type Float%20%28single-precision%29))
  (if (not (Variables|Default|Getopen))
    (Transformation|AddRelativeRotation (Variables|Default|GetSphere) "0.000000,1.000000,0.000000" false false)))

(fn ConstructionScript)